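; MilkJug_Pawn is a physics-driven pawn launched on BeginPlay by an impulse on its Sphere, scaled from a Speed vector.
; Overlapping a "Planet"-tagged actor destroys the first CowPlanet found, not necessarily the one hit, then applies another impulse and compounds Speed.
; Each such boost widens the camera FOV in proportion to Speed's X component.
; Tick prints the current FOV to screen.
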(event OnComponentBeginOverlap(Sphere)
  (params (OverlappedComponent :type Primitive%20Component%20Object%20Reference) (OtherActor :type Actor%20Object%20Reference) (OtherComp :type Primitive%20Component%20Object%20Reference) (OtherBodyIndex :type Integer) (bFromSweep :type Boolean) (SweepResult :type Hit%20Result%20Structure%20%28by%20ref%29))
  (if (Actor|ActorHasTag OtherActor "Planet")
    (bind _returnvalue (Actor|GetActorOfClass "/Game/NewLevel/Blueprints/CowPlanet.CowPlanet_C"))
    (Actor|DestroyActor _returnvalue)
    (Physics|AddImpulse (Variables|Default|GetSphere) (* (Variables|Default|GetSpeed) 1.5) "None" false)
    (Variables|Default|SetSpeed (* (Variables|Default|GetSpeed) 1.5))
    (CallFunction|CameraFOV)))

(event Custom|CameraFOV
  (Camera|SetFieldOfView (Variables|Default|GetCamera) (+ (/ (.x (Variables|Default|GetSpeed)) 4e+03) 9e+01)))

(event EventBeginPlay
  (Physics|AddImpulse (Variables|Default|GetSphere) (* (Variables|Default|GetSpeed) 1.5) "None" false))

(event EventTick
  (params (DeltaSeconds :type Float%20%28single-precision%29))
  (Development|PrintString (Utilities|String|ToString(Float) (Variables|/Script/Engine.CameraComponent|GetFieldOfView (Variables|Default|GetCamera)))))

(fn ConstructionScript)